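; Health component that tracks current and maximum health for its owning actor.
; On BeginPlay it fills Current to Max and binds to the owner's OnTakeAnyDamage event.
; HandleDamage subtracts and clamps health, then broadcasts OnDamage with the remaining fraction while health stays above zero.
; At zero it unbinds from the owner's damage event and broadcasts OnDeath with a zero value.
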(event `self.ReceiveBeginPlay`
  (`self.SetStartHealth`)
  (add `Actor.OnTakeAnyDamage` (`self.GetOwner`) (`|CreateDelegate` :!event `HandleDamage`)))

(event `SetStartHealth`
  (set `self.Current` (`self.Max`)))

(event `HandleDamage`
  (params (DamagedActor :type "Actor Object Reference") (Damage :type "Float (double-precision)") (DamageType :type "DamageType Object Reference") (InstigatedBy :type "Controller Object Reference") (DamageCauser :type "Actor Object Reference"))
  (bind _output_get (set `self.Current` (`KismetMathLibrary.FClamp` (- (`self.Current`) Damage) 0.0 (`self.Max`))))
  (if (> _output_get 0.0)
    (`self.OnDamage` (/ (`self.Current`) (`self.Max`)))
    (else
      (remove `Actor.OnTakeAnyDamage` (`self.GetOwner`) (`|CreateDelegate` :!event `HandleDamage`))
      (`self.OnDeath` 0.0))))