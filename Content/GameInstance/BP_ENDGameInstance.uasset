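; Game instance that handles level flow: loading the first level or main menu, reloading the current level, and quitting the game.
; The load events pass an index to LoadLevelSafe, with the main menu fixed at the first entry of the Levels array.
; LoadLevelSafe validates the index, stores it as CurrentLevel for later reloads and opens that level by name, or prints an error if the index is invalid.
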(event `LoadFirstLevel`
  (`self.LoadLevelSafe` (`self.FirstLevelIndex`)))

(event `QuitGame`
  (`KismetSystemLibrary.QuitGame` null "Quit"))

(event `LoadMainMenu`
  (`self.LoadLevelSafe` 0))

(event `ReloadLevel`
  (`self.LoadLevelSafe` (`self.CurrentLevel`)))

(fn `LoadLevelSafe`
  (params (Index :type Integer))
  (if (`KismetArrayLibrary.Array_IsValidIndex` (`self.Levels`) Index)
    (bind _output_get (set `self.CurrentLevel` Index))
    (`GameplayStatics.OpenLevel` (`|GetArrayItem` (`self.Levels`) _output_get))
    (else
      (`KismetSystemLibrary.PrintString` (`KismetStringLibrary.Concat_StrStr` "Invalid Index " (`KismetStringLibrary.Conv_IntToString` Index))))))