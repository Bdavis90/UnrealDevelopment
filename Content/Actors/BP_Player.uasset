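; BP_Player is the player character, handling camera look, yaw-relative movement and shooting input.
; It creates the WBP_CodeHUD widget on BeginPlay and updates its health when damaged.
; Shooting and character events build on inherited logic: death disables input, plays an animation and removes the HUD, then signals when finished.
; Winning the level also disables input and removes the HUD, stops movement and turns off capsule collision.
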(event `self.ReceiveBeginPlay`
  (`parent.ReceiveBeginPlay`)
  (bind _asplayer_controller (cast `PlayerController` (`self.GetController`))
    (:`then`
      (bind _output_get (set `self.PlayerController` _asplayer_controller))
      (bind _returnvalue (`|CreateWidget` "/Game/Core/Widgets/WBP_CodeHUD.WBP_CodeHUD_C" _output_get))
      (bind _output_get_2 (set `self.HUD` _returnvalue))
      (`UserWidget.AddToViewport` _output_get_2 0))
    (:`CastFailed`
      (`KismetSystemLibrary.PrintString` "Need player controller for HUD"))))

(event `InputAxis|TurnTo`
  (params (AxisValue :type "Float (single-precision)"))
  ;[1 1 1] Rotation
  (`self.AddControllerYawInput` AxisValue))

(event `InputAxis|LookUp`
  (params (AxisValue :type "Float (single-precision)"))
  ;[1 1 1] Rotation
  (`self.AddControllerPitchInput` AxisValue))

(event `InputAxis|MoveForward`
  (params (AxisValue :type "Float (single-precision)"))
  (bind (_returnvalue_roll _returnvalue_pitch _returnvalue_yaw) (`KismetMathLibrary.BreakRotator` (`self.GetControlRotation`)))
  (`self.AddMovementInput` (`KismetMathLibrary.GetForwardVector` (`KismetMathLibrary.MakeRotator` 0.0 0.0 _returnvalue_yaw)) AxisValue))

(event `InputAxis|MoveRight`
  (params (AxisValue :type "Float (single-precision)"))
  (bind (_returnvalue_roll _returnvalue_pitch _returnvalue_yaw) (`KismetMathLibrary.BreakRotator` (`self.GetControlRotation`)))
  (`self.AddMovementInput` (`KismetMathLibrary.GetRightVector` (`KismetMathLibrary.MakeRotator` 0.0 0.0 _returnvalue_yaw)) AxisValue))

(event `InputAction|Shoot`
  (params (Key :type "Key Structure"))
  (:`Pressed`
    (`self.CharacterShoot`)))

(event `self.CharacterDeath`
  (params (Ratio :type "Float (single-precision)"))
  (`self.DisableInput` self (`self.PlayerController`))
  (`parent.CharacterDeath` 0.0)
  (`RifeAnim.PlayDeathAnimation` (`self.AnimBP`) 0.0)
  (`Widget.RemoveFromParent` (`self.HUD`)))

(event `self.CharacterDamaged`
  (params (Ratio :type "Float (single-precision)"))
  (`parent.CharacterDamaged` Ratio)
  (`MyUserWidget.SetHealth` (`self.HUD`) Ratio))

(event `self.CharacterDeathFinished`
  (`parent.CharacterDeathFinished`)
  (`self.OnDeathFinished`))

(event `WonLevel`
  (`self.DisableInput` self (`self.PlayerController`))
  (`Widget.RemoveFromParent` (`self.HUD`))
  (`MovementComponent.StopMovementImmediately` (`self.CharacterMovement`))
  (`PrimitiveComponent.SetCollisionEnabled` (`self.CapsuleComponent`) "NoCollision"))

(fn `UserConstructionScript`
  (`parent.UserConstructionScript`))