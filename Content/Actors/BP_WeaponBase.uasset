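; Base weapon actor that takes its parent actor as the owning pawn and spawns projectiles from the muzzle socket.
; Shoot runs only when neither animating nor dead, then sets the animating lock and fires the OnShoot dispatcher; StopAnimation releases the lock.
; Player shots aim from the muzzle at the first WBP_HUD widget's aimed point, while other pawns, treated as AI, use their base aim rotation.
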(event `self.ReceiveBeginPlay`
  (bind _aspawn (cast `Pawn` (`self.GetParentActor`))
    (:`then`
      (set `self.OwningPawn` _aspawn))
    (:`CastFailed`
      (`KismetSystemLibrary.PrintString` "We need a pawn to own this weapon."))))

(event `Shoot`
  (bind _owningpawn (`self.OwningPawn`))
  (if (`self.CanShoot`)
    (`|SpawnActorFromClass` (`self.ProjectileClass`) (`KismetMathLibrary.MakeTransform` (`SceneComponent.GetSocketLocation` (`self.SkeletalMesh`) "MuzzleFlashSocket") (`self.GetShotRotation`)) "Undefined" "OverrideRootScale" (`Pawn.GetController` _owningpawn) _owningpawn)
    (set `self.Animating` true)
    (`self.OnShoot`)))

(event `StopAnimation`
  (set `self.Animating` false))

(fn `CanShoot`
  (returns (DoShoot :type Boolean))
  (return (and (not (`self.Animating`)) (not (`self.Dead`)))))

(fn `GetShotRotation`
  (returns (Rotation :type "Rotator Structure"))
  (locals (Destination :type "Vector Structure"))
  (bind _foundwidgets (`WidgetBlueprintLibrary.GetAllWidgetsOfClass` "/Game/Core/Widgets/WBP_HUD.WBP_HUD_C" false))
  (bind _output (`|GetArrayItem` _foundwidgets))
  (if (== (`UserWidget.GetOwningPlayerPawn` _output) (`self.OwningPawn`))
    (bind (_valid _hitlocation _endpoint) (`/Game/Core/Widgets/WBP_HUD.Get Aimed Point` _output))
    (if _valid
      (set `local.Destination` _hitlocation)
      (else
        (set `local.Destination` _endpoint)))
    (return (`KismetMathLibrary.MakeRotFromX` (- (`local.Destination`) (`SceneComponent.GetSocketLocation` (`self.SkeletalMesh`) "MuzzleFlashSocket"))))
    (else
      ;[1 1 1] This is the AI
      (return (`Pawn.GetBaseAimRotation` (`self.OwningPawn`))))))

(fn `UserConstructionScript`)